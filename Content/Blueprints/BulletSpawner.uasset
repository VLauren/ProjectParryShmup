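; Bullet spawner actor that repeatedly fires bursts of spread shots toward the player.
; A looping timer started on BeginPlay triggers a burst of three quick volleys, each a three-bullet fan centred on the player.
; SpawnBullet creates a scaled PSBullet and sets its velocity from the player direction, rotated around Z by the given angle.
; The player reference comes from PSGameMode.
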(event `self.ReceiveBeginPlay`
  (`KismetSystemLibrary.K2_SetTimerDelegate` (delegate `Burst`) 2.0 true))

(event `Burst`
  (`self.Shoot`)
  (`KismetSystemLibrary.Delay` 0.15)
  (`self.Shoot`)
  (`KismetSystemLibrary.Delay` 0.15)
  (`self.Shoot`))

(event `Shoot`
  (`self.SpawnBullet` true 0.7 800.0)
  (`self.SpawnBullet` true 0.7 800.0 20.0)
  (`self.SpawnBullet` true 0.7 800.0 -20.0))

(fn `GetDirectionToPlayer`
  (returns (Direction :type "Vector Structure"))
  (bind _aspsgame_mode (cast `/Game/Blueprints/PSGameMode` (`GameplayStatics.GetGameMode`)))
  (bind _res (`/Game/Blueprints/PSGameMode.GetPlayer` _aspsgame_mode))
  (return (`KismetMathLibrary.Normal` (- (`self.K2_GetActorLocation` _res) (`self.K2_GetActorLocation`)))))

(fn `SpawnBullet`
  (params (PlayerRelative :type Boolean) (Size :type "Float (double-precision)") (Speed :type "Float (double-precision)") (Angle :type "Float (double-precision)"))
  (set `self.BaseDir` (0.0 1.0 0.0))
  (if PlayerRelative
    (bind _returnvalue (`|SpawnActorFromClass` "/Game/Blueprints/PSBullet.PSBullet_C" (`KismetMathLibrary.MakeTransform` (`self.K2_GetActorLocation`) (struct) (`KismetMathLibrary.Conv_DoubleToVector` Size)) "Undefined" "OverrideRootScale" null null))
    (bind _direction (`self.GetDirectionToPlayer`))
    (set `self.BaseDir` _direction))
  (set `/Game/Blueprints/PSBullet.Velocity` (`KismetMathLibrary.RotateAngleAxis` (* (`self.BaseDir`) Speed) Angle (0.0 0.0 1.0)) _returnvalue))

(fn `UserConstructionScript`)