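; Base enemy Blueprint with hit points that takes damage from player bullets and dies.
; On overlap with a player bullet, it passes the bullet's damage to Hit and destroys the bullet.
; Hit subtracts damage, prints the remaining HP on screen, and calls Death at zero or below, which destroys the enemy.
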(event `self.ReceiveBeginPlay`
  (set `self.CurrentHitPoints` (`self.MaxHitPoints`)))

(event `self.ReceiveActorBeginOverlap`
  (params (OtherActor :type "Actor Object Reference"))
  (bind _aspsplayer_bullet_base (cast `/Game/Blueprints/Bullets/PSPlayerBulletBase` OtherActor))
  (`self.Hit` (`/Game/Blueprints/Bullets/PSPlayerBulletBase.Damage` _aspsplayer_bullet_base))
  (`self.K2_DestroyActor` _aspsplayer_bullet_base))

(event `Hit`
  (params (Damage :type Integer))
  (bind _output_get (set `self.CurrentHitPoints` (- (`self.CurrentHitPoints`) Damage)))
  (`KismetSystemLibrary.PrintString` (`KismetStringLibrary.Concat_StrStr` "HP: " (`KismetStringLibrary.Conv_IntToString` _output_get)) true true (struct :`R` 0.822917 :`G` 0.734196 :`B` 0.527181 :`A` 0.379))
  (if (<= (`self.CurrentHitPoints`) 0)
    (`self.Death`)))

(event `Death`
  (`self.K2_DestroyActor`))

(fn `UserConstructionScript`)