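; EnemyTest is an enemy Blueprint, apparently for testing, that fires a repeating, timed bullet pattern.
; On BeginPlay it assigns separate burst data to three child-actor BulletSpawners (A, B, C), then starts the pattern immediately and on a looping timer.
; DoShootPattern uses Delays to stagger DoBurst calls, firing C, then B, then A twice within each cycle.
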(event `self.ReceiveBeginPlay`
  (`parent.ReceiveBeginPlay`)
  (bind _asbullet_spawner (cast `/Game/Blueprints/BulletSpawner` (`ChildActorComponent.ChildActor` (`self.BulletSpawnerA`))))
  (set `/Game/Blueprints/BulletSpawner.BurstData` "/Game/Patterns/ShootTest01.ShootTest01" _asbullet_spawner)
  (bind _asbullet_spawner_2 (cast `/Game/Blueprints/BulletSpawner` (`ChildActorComponent.ChildActor` (`self.BulletSpawnerB`))))
  (set `/Game/Blueprints/BulletSpawner.BurstData` "/Game/Patterns/ShootTest02.ShootTest02" _asbullet_spawner_2)
  (bind _asbullet_spawner_3 (cast `/Game/Blueprints/BulletSpawner` (`ChildActorComponent.ChildActor` (`self.BulletSpawnerC`))))
  (set `/Game/Blueprints/BulletSpawner.BurstData` "/Game/Patterns/ShootTest03.ShootTest03" _asbullet_spawner_3)
  (`KismetSystemLibrary.K2_SetTimerDelegate` (delegate `DoShootPattern`) 9.0 true)
  (`self.DoShootPattern`))

(event `DoShootPattern`
  (bind _asbullet_spawner (cast `/Game/Blueprints/BulletSpawner` (`ChildActorComponent.ChildActor` (`self.BulletSpawnerC`))))
  (`/Game/Blueprints/BulletSpawner.DoBurst` _asbullet_spawner)
  (`KismetSystemLibrary.Delay` 2.0)
  (bind _asbullet_spawner_2 (cast `/Game/Blueprints/BulletSpawner` (`ChildActorComponent.ChildActor` (`self.BulletSpawnerB`))))
  (`/Game/Blueprints/BulletSpawner.DoBurst` _asbullet_spawner_2)
  (`KismetSystemLibrary.Delay` 4.0)
  (bind _asbullet_spawner_3 (cast `/Game/Blueprints/BulletSpawner` (`ChildActorComponent.ChildActor` (`self.BulletSpawnerA`))))
  (`/Game/Blueprints/BulletSpawner.DoBurst` _asbullet_spawner_3)
  (`KismetSystemLibrary.Delay` 1.0)
  (bind _asbullet_spawner_4 (cast `/Game/Blueprints/BulletSpawner` (`ChildActorComponent.ChildActor` (`self.BulletSpawnerA`))))
  (`/Game/Blueprints/BulletSpawner.DoBurst` _asbullet_spawner_4))

(fn `UserConstructionScript`
  (`parent.UserConstructionScript`))