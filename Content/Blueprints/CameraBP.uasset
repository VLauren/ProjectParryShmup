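; CameraBP is a camera actor that follows the player with damped horizontal movement.
; On BeginPlay it stores its offset from the first PlayerBP in the level.
; Each Tick it reads the player location from PSGameMode and adds that offset, scaling player X to one third, tracking Z fully and holding Y at the offset value.
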(event `self.ReceiveBeginPlay`
  (bind _outactors (`GameplayStatics.GetAllActorsOfClass` "/Game/Blueprints/PlayerBP.PlayerBP_C"))
  (bind _output_get (set `self.Player` (`|GetArrayItem` _outactors)))
  (set `self.Offset` (- (`self.K2_GetActorLocation`) (`self.K2_GetActorLocation` _output_get))))

(event `self.ReceiveTick`
  (params (DeltaSeconds :type "Float (single-precision)"))
  (bind _y (.y (`self.Offset`)))
  (bind _aspsgame_mode (cast `/Game/Blueprints/PSGameMode` (`GameplayStatics.GetGameMode`)))
  (bind _location (`/Game/Blueprints/PSGameMode.GetPlayerLocation` _aspsgame_mode))
  (bind (_returnvalue_x _returnvalue_y _returnvalue_z) (`KismetMathLibrary.BreakVector` (+ (`KismetMathLibrary.MakeVector` (.x (`self.Offset`)) _y (.z (`self.Offset`))) (`KismetMathLibrary.MakeVector` (/ (.x _location) 3.0) 0.0 (.z _location)))))
  (`self.K2_SetActorLocation` (`KismetMathLibrary.MakeVector` _returnvalue_x _y _returnvalue_z)))

(fn `UserConstructionScript`)