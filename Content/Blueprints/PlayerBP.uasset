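; Player ship Blueprint for a shoot-'em-up: moves within fixed X/Y bounds, fires bursts and dies on enemy bullets.
; Tick calls Movimiento for normalized, speed-scaled movement, tilting the actor with horizontal input.
; Input A triggers bursts on a child-actor BulletSpawner configured at BeginPlay.
; Enemy bullet overlaps notify PSGameMode and destroy the player, except during debug or timed spawn invulnerability, the latter shown by a looping mesh blink.
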(event `self.ReceiveBeginPlay`
  (bind _asbullet_spawner (cast `/Game/Blueprints/BulletSpawner` (`ChildActorComponent.ChildActor` (`self.BulletSpawnA`))))
  (set `/Game/Blueprints/BulletSpawner.BurstData` "/Game/Patterns/PlayerShootTestA.PlayerShootTestA" _asbullet_spawner)
  (`self.InvulBlink`)
  (`KismetSystemLibrary.Delay` 2.5) ; Tiempo de invulnerabilidad al spawnear
  (set `self.SpawnInvulnerable` false)
  (`SceneComponent.SetVisibility` (`self.Mesh`) true false))

(event `self.ReceiveTick`
  (params (DeltaSeconds :type "Float (single-precision)"))
  (`self.Movimiento` DeltaSeconds))

(event `InputAction|A`
  (params (Key :type "Key Structure"))
  (:`Pressed`
    (bind _asbullet_spawner (cast `/Game/Blueprints/BulletSpawner` (`ChildActorComponent.ChildActor` (`self.BulletSpawnA`))))
    (`/Game/Blueprints/BulletSpawner.DoBurst` _asbullet_spawner)))

(event `self.ReceiveActorBeginOverlap`
  (params (OtherActor :type "Actor Object Reference"))
  (cast `/Game/Blueprints/PSEnemyBullet` OtherActor)
  (`KismetSystemLibrary.PrintString` (`KismetStringLibrary.Concat_StrStr` "Colision con " (`KismetSystemLibrary.GetDisplayName` OtherActor) "!") true true (struct :`R` 1.0 :`G` 0.209649 :`A` 1.0))
  (if (not (or (`self.DebugInvulnerable`) (`self.SpawnInvulnerable`)))
    (bind _aspsgame_mode (cast `/Game/Blueprints/PSGameMode` (`GameplayStatics.GetGameMode`)))
    (`/Game/Blueprints/PSGameMode.Player Death` _aspsgame_mode)
    (`self.K2_DestroyActor`)))

(event `InvulBlink`
  ;[1 1 1] Parpadeo invulnerabilidad
  (`SceneComponent.SetVisibility` (`self.Mesh`) true false :!label _label)
  (`KismetSystemLibrary.Delay` 0.15)
  (if (`self.SpawnInvulnerable`)
    (`SceneComponent.SetVisibility` (`self.Mesh`) false false)
    (`KismetSystemLibrary.Delay` 0.1)
    (goto _label)))

(fn `Movimiento`
  (params (`Delta Seconds` :type "Float (double-precision)"))
  (bind _output_get (set `self.NewLoc` (+ (`self.K2_GetActorLocation`) (* (`KismetMathLibrary.Normal` (`KismetMathLibrary.MakeVector` (`self.GetInputAxisValue`) (* (`self.GetInputAxisValue`) -1.0))) (* `Delta Seconds` (`self.Speed`))))))
  (`self.K2_SetActorLocation` (`KismetMathLibrary.MakeVector` (`KismetMathLibrary.FClamp` (.x _output_get) (`self.XMin`) (`self.XMax`)) (`KismetMathLibrary.FClamp` (.y _output_get) (`self.YMin`) (`self.YMax`)) (.z _output_get)))
  (`self.K2_SetActorRotation` (`KismetMathLibrary.MakeRotator` 0.0 (select `bool` (< (`self.GetInputAxisValue`) 0.0) :`false` (select `bool` (> (`self.GetInputAxisValue`) 0.0) :`true` -30.0 :!type "Float (single-precision)") :`true` 30.0))))

(fn `UserConstructionScript`)