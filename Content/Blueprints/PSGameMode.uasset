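; Game mode Blueprint that tracks the player and respawns it after death.
; Tick caches the player's location each frame, found through GetPlayer, which lazily finds and stores the first PlayerBP actor.
; PlayerDeath waits briefly, then spawns a new PlayerBP at that last known location.
; GetPlayerLocation returns the live position, falling back to the cached one while no player exists.
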(event `self.ReceiveBeginPlay`)

(event `self.ReceiveTick`
  (params (DeltaSeconds :type "Float (single-precision)"))
  (bind _res (`self.GetPlayer`))
  (if (`KismetSystemLibrary.IsValid` _res)
    (set `self.LastPlayerLocation` (`self.K2_GetActorLocation` _res))))

(event `Player Death`
  (`KismetSystemLibrary.Delay` 1.0) ; Tiempo entre muerte y spawn
  (`|SpawnActorFromClass` "/Game/Blueprints/PlayerBP.PlayerBP_C" (`KismetMathLibrary.MakeTransform` (`self.LastPlayerLocation`)) "Undefined" "OverrideRootScale" null null))

(fn `GetPlayer`
  (returns (Res :type "/Game/Blueprints/PlayerBP Object Reference"))
  (if (not (`KismetSystemLibrary.IsValid` (`self.PlayerRef`)))
    (bind _outactors (`GameplayStatics.GetAllActorsOfClass` "/Game/Blueprints/PlayerBP.PlayerBP_C"))
    (if (> (`KismetArrayLibrary.Array_Length` _outactors) 0)
      (set `self.PlayerRef` (`|GetArrayItem` _outactors))
      (else
        (set `self.PlayerRef` null))))
  (return (`self.PlayerRef`)))

(fn `GetPlayerLocation`
  (returns (Location :type "Vector Structure"))
  (bind _res (`self.GetPlayer`))
  (if (`KismetSystemLibrary.IsValid` _res)
    (return (`self.K2_GetActorLocation` _res))
    (else
      (return (`self.LastPlayerLocation`)))))

(fn `UserConstructionScript`)